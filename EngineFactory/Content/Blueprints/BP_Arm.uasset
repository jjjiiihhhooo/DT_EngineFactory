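; BP_Arm is a robot arm actor whose end control follows a scene component through Control Rig.
; On BeginPlay it maps the skeletal mesh to the rig as output and moves that scene component to a default relative position.
; Each tick it writes the component's world location to the end control.
; A StateChange event passes the acting state to a WBP_ArmState widget to update its text.
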(event `self.ReceiveBeginPlay`
  (bind _returnvalue_location (`KismetMathLibrary.BreakTransform` (`SceneComponent.GetRelativeTransform` (`self.Default`))))
  (set `self.Point` (`self.Scene`))
  (`ControlRigComponent.AddMappedCompleteSkeletalMesh` (`self.ControlRig`) (`self.SkeletalMesh`) "Output")
  (`SceneComponent.K2_SetRelativeLocation` (`self.Scene`) _returnvalue_location false false))

(event `self.ReceiveTick`
  (params (DeltaSeconds :type "Float (single-precision)"))
  (`ControlRigComponent.SetControlTransform` (`self.ControlRig`) "Robot1_End_Control" (`KismetMathLibrary.MakeTransform` (`SceneComponent.K2_GetComponentLocation` (`self.Scene`))) "WorldSpace"))

(event `self.StateChange`
  (params (acting :type Boolean))
  (bind _aswbp_arm_state (cast `/Game/Blueprints/WBP_ArmState` (`WidgetComponent.GetUserWidgetObject` (`self.Widget`))))
  (`/Game/Blueprints/WBP_ArmState.SetStateText` _aswbp_arm_state acting))

(fn `UserConstructionScript`)