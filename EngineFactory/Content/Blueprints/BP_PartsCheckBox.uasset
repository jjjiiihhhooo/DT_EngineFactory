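; BP_PartsCheckBox is a trigger gate that takes in overlapping EngineParts actors and reports them for counting.
; On BeginPlay it passes its Name to the WBP_Gate widget.
; On overlap it stops the part's movement, hands it to BP_PartsSpawner via ReturnParts, and sends its PartsIndex to BP_Manager's AddCountEvent.
; It finds the spawner and manager with GetAllActorsOfClass on each overlap, using the first result.
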(event `self.ReceiveBeginPlay`
  (bind _aswbp_gate (cast `/Game/Blueprints/WBP_Gate` (`WidgetComponent.GetWidget` (`self.Widget`))))
  (`/Game/Blueprints/WBP_Gate.SetNameEvent` _aswbp_gate (`self.Name`)))

(event `self.Trigger.OnComponentBeginOverlap`
  (params (OverlappedComponent :type "PrimitiveComponent Object Reference") (OtherActor :type "Actor Object Reference") (OtherComp :type "PrimitiveComponent Object Reference") (OtherBodyIndex :type Integer) (bFromSweep :type Boolean) (SweepResult :type "HitResult Structure (by ref)"))
  (bind _asengine_parts (cast `EngineParts` OtherActor))
  (`EngineParts.SetCanMove` _asengine_parts false)
  (bind _outactors (`GameplayStatics.GetAllActorsOfClass` "/Game/Blueprints/BP_PartsSpawner.BP_PartsSpawner_C"))
  (bind _partsindex (`EngineParts.PartsIndex` _asengine_parts))
  (`Spawner.ReturnParts` (`|GetArrayItem` _outactors) _asengine_parts _partsindex)
  (bind _outactors_2 (`GameplayStatics.GetAllActorsOfClass` "/Game/Blueprints/BP_Manager.BP_Manager_C"))
  (`/Game/Blueprints/BP_Manager.AddCountEvent` (`|GetArrayItem` _outactors_2) _partsindex))

(fn `UserConstructionScript`)