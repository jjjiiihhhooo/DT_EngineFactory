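; BP_Manager is a manager Blueprint that sets up the game's UI and relays count and exit-menu events.
; On BeginPlay it shows the mouse cursor and adds the camera control, factory manager and exit menu widgets to the viewport, hiding the exit menu.
; AddCountEvent increments a count by index and pushes the new value to the factory manager widget.
; Other events show or hide the exit menu and quit the game.
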(event `self.ReceiveBeginPlay`
  (bind _returnvalue (`GameplayStatics.GetPlayerController` 0))
  (set `PlayerController.bShowMouseCursor` true _returnvalue)
  (`|ExecutionSequence`
    (:`then_0`
      (bind _returnvalue_2 (`|CreateWidget` "/Game/Blueprints/WBP_Camera_Control.WBP_Camera_Control_C" _returnvalue))
      (`UserWidget.AddToViewport` _returnvalue_2 1))
    (:`then_1`
      (bind _returnvalue_3 (`|CreateWidget` "/Game/Blueprints/WBP_FactoryManager.WBP_FactoryManager_C" _returnvalue))
      (bind _output_get (set `self.WBP_FactoryManager` _returnvalue_3))
      (`UserWidget.AddToViewport` _output_get 0))
    (:`then_2`
      (bind _returnvalue_4 (`|CreateWidget` "/Game/Blueprints/WBP_ExitMenu.WBP_ExitMenu_C" _returnvalue))
      (bind _output_get_2 (set `self.Exit Menu Widget` _returnvalue_4))
      (`UserWidget.AddToViewport` _returnvalue_4 2)
      (`Widget.SetVisibility` _output_get_2 "Hidden"))))

(event `AddCountEvent`
  (params (Index :type Integer))
  (`self.AddCountByIndex` Index)
  (bind _returnvalue (`self.GetCountByIndex` Index))
  (`/Game/Blueprints/WBP_FactoryManager.SetCountTextEvent` (`self.WBP_FactoryManager`) Index _returnvalue))

(event `OpenExitMenu`
  (`Widget.SetVisibility` (`self.Exit Menu Widget`) "Visible"))

(event `CloseExitMenu`
  (`Widget.SetVisibility` (`self.Exit Menu Widget`) "Hidden"))

(event `ExitGameEvent`
  (`KismetSystemLibrary.QuitGame` null "Quit"))

(fn `UserConstructionScript`)